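; DeathZone is a hazard actor for a side-scroller that respawns the player and kills weak enemies on contact.
; Its Cube's hit event casts the other actor to SideScrollChar, subtracting a small amount of Health and calling Respawn.
; Otherwise, a WeakEnemy has its Health zeroed and is destroyed, and the player 0 pawn gains experience points, regardless of what caused the enemy to hit the zone.
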(event `self.Cube.OnComponentHit`
  (params (HitComponent :type "PrimitiveComponent Object Reference") (OtherActor :type "Actor Object Reference") (OtherComp :type "PrimitiveComponent Object Reference") (NormalImpulse :type "Vector Structure") (Hit :type "HitResult Structure (by ref)"))
  (bind _asside_scroll_char (cast `/Game/Blueprints/SideScrollChar` OtherActor)
    (:`then`
      (set `/Game/Blueprints/SideScrollChar.Health` (- (`/Game/Blueprints/SideScrollChar.Health` _asside_scroll_char) 0.1) _asside_scroll_char)
      (`/Game/Blueprints/SideScrollChar.Respawn` _asside_scroll_char))
    (:`CastFailed`
      (bind _asweak_enemy (cast `/Game/Blueprints/WeakEnemy` OtherActor))
      (set `/Game/Blueprints/WeakEnemy.Health` 0 _asweak_enemy)
      (`self.K2_DestroyActor` _asweak_enemy)
      (bind _asside_scroll_char_2 (cast `/Game/Blueprints/SideScrollChar` (`GameplayStatics.GetPlayerPawn` 0)))
      (set `/Game/Blueprints/SideScrollChar.ExperiencePoints` (+ (`/Game/Blueprints/SideScrollChar.ExperiencePoints` _asside_scroll_char_2) 300) _asside_scroll_char_2))))

(fn `UserConstructionScript`)