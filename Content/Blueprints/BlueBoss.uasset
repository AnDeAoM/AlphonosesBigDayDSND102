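; Blue boss enemy character for a side-scroller that chases the player whenever Pawn Sensing spots a pawn and it is not stunned.
; Capsule hits on the player knock them back, deal boss damage and trigger a one-second cooldown stun.
; Knockback subtracts the player's STR from Health, then either launches the boss or destroys it, granting experience and a skill point.
; A separate Stunned event duplicates the cooldown logic.
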(event `self.ReceiveTick`
  (params (DeltaSeconds :type "Float (single-precision)")))

(event `self.PawnSensing.OnSeePawn`
  (params (Pawn :type "Pawn Object Reference"))
  (if (not (`self.EnemyStunned`))
    (`|AIMoveTo` self (0.0 0.0 0.0) (`GameplayStatics.GetPlayerPawn` 0))))

(event `Stunned`
  (set `self.EnemyStunned` true)
  (`MovementComponent.StopMovementImmediately` (`self.CharacterMovement`))
  (`KismetSystemLibrary.Delay` 1.0)
  (set `self.EnemyStunned` false))

(event `CoolDown`
  (set `self.EnemyStunned` true)
  (`MovementComponent.StopMovementImmediately` (`self.CharacterMovement`))
  (`KismetSystemLibrary.Delay` 1.0)
  (set `self.EnemyStunned` false))

(event `self.CapsuleComponent.OnComponentHit`
  (params (HitComponent :type "PrimitiveComponent Object Reference") (OtherActor :type "Actor Object Reference") (OtherComp :type "PrimitiveComponent Object Reference") (NormalImpulse :type "Vector Structure") (Hit :type "HitResult Structure (by ref)"))
  (bind _asside_scroll_char (cast `/Game/Blueprints/SideScrollChar` OtherActor))
  (`/Game/Blueprints/SideScrollChar.PlayerKnockBack` _asside_scroll_char (`self.GetActorForwardVector`))
  (`/Game/Blueprints/SideScrollChar.BlueBossDamage` _asside_scroll_char)
  (`self.CoolDown`))

(event `Knockback`
  (params (NewParam :type "Vector Structure"))
  (bind _health (`self.Health`))
  (bind _asside_scroll_char (cast `/Game/Blueprints/SideScrollChar` (`GameplayStatics.GetPlayerPawn` 0)))
  (set `self.Health` (- _health (`/Game/Blueprints/SideScrollChar.STR` _asside_scroll_char)))
  (if (<= _health 0)
    (`self.K2_DestroyActor`)
    (set `/Game/Blueprints/SideScrollChar.ExperiencePoints` (+ (`/Game/Blueprints/SideScrollChar.ExperiencePoints` _asside_scroll_char) 1000) _asside_scroll_char)
    (`/Game/Blueprints/SideScrollChar.addSkillPoint` _asside_scroll_char)
    (else
      (`self.LaunchCharacter` (* NewParam (1000.0 1000.0 0.0))))))

(fn `UserConstructionScript`)