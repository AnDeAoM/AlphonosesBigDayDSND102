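; Projectile that flies from the player side-scroller character and knocks back the enemies it hits.
; On BeginPlay it sets its local-space velocity from the forward vector of the player's Properspawn component.
; When its sphere hits, a cast chain checks for a weak enemy or one of four bosses, calls that class's Knockback and destroys the projectile.
; Any other hit destroys it after a short delay.
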(event `self.Sphere.OnComponentHit`
  (params (HitComponent :type "PrimitiveComponent Object Reference") (OtherActor :type "Actor Object Reference") (OtherComp :type "PrimitiveComponent Object Reference") (NormalImpulse :type "Vector Structure") (Hit :type "HitResult Structure (by ref)"))
  (bind _forwardvector (`self.ForwardVector`))
  (bind _asweak_enemy (cast `/Game/Blueprints/WeakEnemy` OtherActor)
    (:`then`
      (`/Game/Blueprints/WeakEnemy.Knockback` _asweak_enemy _forwardvector)
      (`self.K2_DestroyActor`))
    (:`CastFailed`
      (bind _asblue_boss (cast `/Game/Blueprints/BlueBoss` OtherActor)
        (:`then`
          (`/Game/Blueprints/BlueBoss.Knockback` _asblue_boss _forwardvector)
          (`self.K2_DestroyActor`))
        (:`CastFailed`
          (bind _aspinkboss (cast `/Game/Blueprints/Pinkboss` OtherActor)
            (:`then`
              (`/Game/Blueprints/Pinkboss.Knockback` _aspinkboss _forwardvector)
              (`self.K2_DestroyActor`))
            (:`CastFailed`
              (bind _asgreen_boss (cast `/Game/Blueprints/GreenBoss` OtherActor)
                (:`then`
                  (`/Game/Blueprints/GreenBoss.Knockback` _asgreen_boss _forwardvector)
                  (`self.K2_DestroyActor`))
                (:`CastFailed`
                  (bind _asfinal_boss (cast `/Game/Blueprints/FinalBoss` OtherActor)
                    (:`then`
                      (`/Game/Blueprints/FinalBoss.Knockback` _asfinal_boss _forwardvector)
                      (`self.K2_DestroyActor`))
                    (:`CastFailed`
                      (`KismetSystemLibrary.Delay` 5.0)
                      (`self.K2_DestroyActor`))))))))))))

(event `self.ReceiveBeginPlay`
  (bind _asside_scroll_char (cast `/Game/Blueprints/SideScrollChar` (`GameplayStatics.GetPlayerPawn` 0)))
  (`ProjectileMovementComponent.SetVelocityInLocalSpace` (`self.ProjectileMovement`) (* (`SceneComponent.GetForwardVector` (`/Game/Blueprints/SideScrollChar.properspawn` _asside_scroll_char)) (1000.0 1000.0 1000.0))))

(fn `UserConstructionScript`)